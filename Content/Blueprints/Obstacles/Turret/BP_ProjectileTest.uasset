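; BP_ProjectileTest is a turret obstacle projectile that deals damage to whatever it overlaps, ignoring other projectiles of its own class.
; Each tick it sets its movement component velocity along its forward vector at ProjectileSpeed.
; On a hit it calls Deactivate, then applies damage.
; Activate, deactivate and transform-update functions support reuse without destruction by toggling visibility, tick and collision, with deactivation also moving it below the origin.
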(event EventBeginPlay)

(event Collision|EventActorBeginOverlap
  (params (OtherActor :type Actor%20Object%20Reference))
  (Utilities|Casting|CastToBP_ProjectileTest OtherActor
    (:CastFailed
      (CallFunction|Deactivate)
      (Game|Damage|ApplyDamage OtherActor 1.0 0 0))))

(event EventTick
  (params (DeltaSeconds :type Float%20%28single-precision%29))
  (Variables|/Script/Engine.MovementComponent|SetVelocity (Variables|Default|GetProjectileMovement) (* (Transformation|GetActorForwardVector) (Variables|Default|GetProjectileSpeed))))

(fn ConstructionScript)

(fn BPActivate
  (Rendering|SetActorHiddenInGame false)
  (Actor|Tick|SetActorTickEnabled true)
  (Collision|SetActorEnableCollision true))

(fn BPDeactivate
  (Transformation|SetActorLocation "0.000000,0.000000,-100.000000" false false)
  (Rendering|SetActorHiddenInGame true)
  (Actor|Tick|SetActorTickEnabled false)
  (Collision|SetActorEnableCollision false))

(fn BPUpdateTransform
  (params (GivenTransform :type Transform) (IsSweep :type Boolean))
  (Transformation|SetActorTransform GivenTransform IsSweep))