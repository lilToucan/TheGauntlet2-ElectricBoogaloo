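; Turret obstacle Blueprint that configures a turret component and a flickering-light component.
; The construction script copies Range and FireRate into TurretComponent and hands the Light mesh to FlickLightComponent.
; It also previews the search radius with a long-lived debug sphere, flushing all persistent debug lines before each redraw.
; The event graph adds no logic of its own, only forwarding BeginPlay and Tick to the parent.
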(event EventBeginPlay
  (|CallParentFunction))

(event Collision|EventActorBeginOverlap
  (params (OtherActor :type Actor%20Object%20Reference)))

(event EventTick
  (params (DeltaSeconds :type Float%20%28single-precision%29))
  (|CallParentFunction DeltaSeconds))

(fn ConstructionScript
  (Rendering|Debug|FlushPersistentDebugLines)
  (bind _output_get (Variables|/Script/TheGauntlet_2.TurretComponent|SetSearchRadius (Variables|Default|GetTurretComponent) (Variables|Default|GetRange)))
  (Rendering|Debug|DrawDebugSphere (Transformation|GetActorLocation) _output_get 12 "(R=0.002686,G=0.140625,B=0.027716,A=1.000000)" 999999999999.0)
  (Variables|/Script/TheGauntlet_2.TurretComponent|SetFireRate (Variables|Default|GetTurretComponent) (Variables|Default|GetFireRate))
  (Variables|/Script/TheGauntlet_2.FlickLightComponent|SetMesh (Variables|Default|GetFlickLightComponent) (Variables|Default|GetLight)))