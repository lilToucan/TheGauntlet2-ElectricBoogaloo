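; BP_WinCollider is a win trigger that returns the game to the main menu after an overlap lasts two seconds.
; Overlap begin sets a flag, and Tick accumulates time while it is set; overlap end clears the flag and resets the timer.
; At the threshold it calls LoadLevel on BP_GauntletGameInstance to load MainMenu.
; Neither overlap event checks which actor is involved.
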(event EventBeginPlay)

(event Collision|EventActorBeginOverlap
  (params (OtherActor :type Actor%20Object%20Reference))
  (Variables|Default|SetIsOverlapping true))

(event EventTick
  (params (DeltaSeconds :type Float%20%28single-precision%29))
  (if (Variables|Default|GetIsOverlapping)
    (bind _output_get (Variables|Default|Settimer (+ (Variables|Default|Gettimer) DeltaSeconds)))
    (if (>= _output_get 2.0)
      (bind _asbp_gauntlet_game_instance (Utilities|Casting|CastToBP_GauntletGameInstance (Game|GetGameInstance)))
      (Class|GauntletGameInstance|LoadLevel _asbp_gauntlet_game_instance "/Game/Levels/MainMenu.MainMenu"))))

(event Collision|EventActorEndOverlap
  (params (OtherActor :type Actor%20Object%20Reference))
  (Variables|Default|Settimer 0.0)
  (Variables|Default|SetIsOverlapping false))

(fn ConstructionScript)