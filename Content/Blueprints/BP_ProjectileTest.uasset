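; BP_ProjectileTest is a test projectile actor that is switched on and off in place rather than spawned or destroyed.
; BP_Activate and BP_Deactivate toggle visibility, tick and collision together, a pattern suited to object pooling.
; BP_UpdateTransform moves the actor to a given transform with optional sweep and no teleport.
; Any actor overlap calls Deactivate, which is not defined in this Blueprint.
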(event EventBeginPlay)

(event Collision|EventActorBeginOverlap
  (params (OtherActor :type Actor%20Object%20Reference))
  (CallFunction|Deactivate))

(event EventTick
  (params (DeltaSeconds :type Float%20%28single-precision%29)))

(fn ConstructionScript)

(fn BPActivate
  (Rendering|SetActorHiddenInGame false)
  (Actor|Tick|SetActorTickEnabled true)
  (Collision|SetActorEnableCollision true))

(fn BPDeactivate
  (Rendering|SetActorHiddenInGame true)
  (Actor|Tick|SetActorTickEnabled false)
  (Collision|SetActorEnableCollision false))

(fn BPUpdateTransform
  (params (GivenTransform :type Transform) (IsSweep :type Boolean))
  (Transformation|SetActorTransform GivenTransform IsSweep))